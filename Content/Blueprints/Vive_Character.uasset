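; VR player character for Vive motion controllers, with grip pickup and left-hand teleport.
; While a grip is held, hand mesh hits snap BI_Pickup components to that hand's socket; release detaches the shared PickedObject and enables physics.
; Holding the left trigger runs a gated retriggerable-delay trace loop that marks flat ground with a debug cylinder.
; Releasing it moves the capsule there, offset for the camera's horizontal position.
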(event OnComponentHit(L_HandMesh)
  (params (OtherActor :type Actor%20Object%20Reference) (OtherComp :type Primitive%20Component%20Object%20Reference) (NormalImpulse :type Vector :default "0, 0, 0") (Hit :type Hit%20Result%20Structure%20%28by%20ref%29))
  ;[1 1 1] PickUP
  (if (and (Utilities|DoesObjectImplementInterface OtherActor "/Game/Interfaces/BI_Pickup.BI_Pickup_C") (Variables|Default|GetbLGripPressed))
    (Class|SceneComponent|Attachto OtherComp (Variables|Default|GetL_HandMesh) "L_HoldObject" "SnapToTarget" true)
    (Variables|Default|SetPickedObject OtherComp)))

(event OnComponentHit(R_HandMesh)
  (params (OtherActor :type Actor%20Object%20Reference) (OtherComp :type Primitive%20Component%20Object%20Reference) (NormalImpulse :type Vector :default "0, 0, 0") (Hit :type Hit%20Result%20Structure%20%28by%20ref%29))
  ;[1 1 1] PickUP
  (if (and (Utilities|DoesObjectImplementInterface OtherActor "/Game/Interfaces/BI_Pickup.BI_Pickup_C") (Variables|Default|GetbRGripPressed))
    (Class|SceneComponent|Attachto OtherComp (Variables|Default|GetR_HandMesh) "HoldObjecte" "SnapToTarget" true)
    (Variables|Default|SetPickedObject OtherComp)))

(event Custom|Move
  ;[1 1 1] Move
  (Transformation|SetWorldLocation (Variables|Collision|GetCapsuleComponent) (Variables|Default|GetTele_Location) false false))

(event Custom|EndTeleport
  (bind _camera (Variables|Default|GetCamera))
  (bind _capsulecomponent (Variables|Collision|GetCapsuleComponent))
  (bind _l_motioncontroller (Variables|Default|GetL_MotionController))
  (bind _returnvalue (Transformation|GetWorldLocation _camera))
  (bind _returnvalue_2 (Transformation|GetWorldLocation _capsulecomponent))
  (bind _returnvalue_3 (Transformation|GetWorldLocation _l_motioncontroller))
  (bind _returnvalue_4 (Transformation|GetWorldRotation _l_motioncontroller))
  (bind _returnvalue_5 (- _returnvalue _returnvalue_2))
  (bind _returnvalue_6 (Math|Vector|GetForwardVector _returnvalue_4))
  (bind (_x _y) (Math|Vector|BreakVector _returnvalue_5))
  ;[1 1 1] Teleprot
  (Utilities|FlowControl|Gate true) ; enters at Close
)

(event Custom|StartTeleport
  (bind _camera (Variables|Default|GetCamera))
  (bind _capsulecomponent (Variables|Collision|GetCapsuleComponent))
  (bind _l_motioncontroller (Variables|Default|GetL_MotionController))
  (bind _returnvalue (Transformation|GetWorldLocation _camera))
  (bind _returnvalue_2 (Transformation|GetWorldLocation _capsulecomponent))
  (bind _returnvalue_3 (Transformation|GetWorldLocation _l_motioncontroller))
  (bind _returnvalue_4 (Transformation|GetWorldRotation _l_motioncontroller))
  (bind _returnvalue_5 (- _returnvalue _returnvalue_2))
  (bind _returnvalue_6 (Math|Vector|GetForwardVector _returnvalue_4))
  (bind (_x _y) (Math|Vector|BreakVector _returnvalue_5))
  ;[1 1 1] Teleprot
  (Utilities|FlowControl|Sequence
    (:then_0
      (goto _label Open))
    (:then_1
      (Utilities|FlowControl|Gate true :!label _label
        (:Exit
          (Utilities|FlowControl|Sequence
            (:then_0
              (bind (_outhit _returnvalue_7) (Collision|LineTraceByChannel (+ _returnvalue_3 _returnvalue_6) (+ _returnvalue_3 (* _returnvalue_6 (Math|Conversions|ToFloat(Integer) (Variables|Default|GetTeleport_Distance)))) "TraceTypeQuery1" false 0 "ForOneFrame"))
              (if _returnvalue_7
                (if (> (Math|Vector|DotProduct (.Normal (Collision|BreakHitResult _outhit)) "0, 0,1.000000") 0.9)
                  (Variables|Default|SetTele_Location (- (.Location (Collision|BreakHitResult _outhit)) (Math|Vector|MakeVector _x _y 0.0)))
                  (Class|KismetSystemLibrary|DrawDebugCylinder (.Location (Collision|BreakHitResult _outhit)) (+ (.Location (Collision|BreakHitResult _outhit)) (* (.Normal (Collision|BreakHitResult _outhit)) 20)) 2e+01 12 "(R=0.800000,G=0.159085,B=0.143805,A=1.000000)" 0.0))))
            (:then_1
              (Utilities|FlowControl|RetriggerableDelay 0.01)
              (goto _label))))))))

(event Input|KeyboardEvents|MotionControllerLeftTrigger
  (params (Key :type Key%20Structure :default "AnyKey"))
  (:Pressed
    (CallFunction|StartTeleport))
  (:Released
    (CallFunction|Move)
    (CallFunction|EndTeleport)))

(event Input|KeyboardEvents|MotionControllerLeftGrip1
  (params (Key :type Key%20Structure :default "AnyKey"))
  (bind _pickedobject (Variables|Default|GetPickedObject))
  ;[1 1 1] PickUP
  (:Pressed
    (Variables|Default|SetbLGripPressed true))
  (:Released
    (Variables|Default|SetbLGripPressed false)
    (Class|SceneComponent|DetachfromParent _pickedobject false true)
    (Physics|SetSimulatePhysics _pickedobject true)))

(event Input|KeyboardEvents|MotionControllerLeftGrip2
  (params (Key :type Key%20Structure :default "AnyKey"))
  (bind _pickedobject (Variables|Default|GetPickedObject))
  ;[1 1 1] PickUP
  (:Pressed
    (Variables|Default|SetbLGripPressed true))
  (:Released
    (Variables|Default|SetbLGripPressed false)
    (Class|SceneComponent|DetachfromParent _pickedobject false true)
    (Physics|SetSimulatePhysics _pickedobject true)))

(event Input|KeyboardEvents|MotionControllerRightGrip1
  (params (Key :type Key%20Structure :default "AnyKey"))
  (bind _pickedobject (Variables|Default|GetPickedObject))
  ;[1 1 1] PickUP
  (:Pressed
    (Variables|Default|SetbRGripPressed true))
  (:Released
    (Variables|Default|SetbRGripPressed false)
    (Class|SceneComponent|DetachfromParent _pickedobject false true)
    (Physics|SetSimulatePhysics _pickedobject true)))

(event Input|KeyboardEvents|MotionControllerRightGrip2
  (params (Key :type Key%20Structure :default "AnyKey"))
  (bind _pickedobject (Variables|Default|GetPickedObject))
  ;[1 1 1] PickUP
  (:Pressed
    (Variables|Default|SetbRGripPressed true))
  (:Released
    (Variables|Default|SetbRGripPressed false)
    (Class|SceneComponent|DetachfromParent _pickedobject false true)
    (Physics|SetSimulatePhysics _pickedobject true)))

(fn ConstructionScript)